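; BP_DualToughSwords is a dual-sword weapon actor in the combat system that deals point damage to what its collision components hit.
; Hit events from the RightFoot and OffHandWeaponCollisionComponent components run identical logic, first checking whether the hit actor can receive damage.
; Valid hits apply GetDamage along the owner's forward vector, crediting the instigator controller, with the weapon as damage causer.
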(event OnHit(RightFoot)
  (params (HitResult :type Hit%20Result%20Structure))
  (bind _hitactor (Collision|BreakHitResult HitResult))
  (bind _returnvalue (Class|CombatBPI|CanReceiveDamage(Message) _hitactor))
  (if _returnvalue
    (Game|Damage|ApplyPointDamage _hitactor (CallFunction|GetDamage) (Transformation|GetActorForwardVector (Components|GetOwner)) HitResult (Game|GetInstigatorController) self)))

(event OnHit(Off-HandWeaponCollisionComponent)
  (params (HitResult :type Hit%20Result%20Structure))
  (bind _hitactor (Collision|BreakHitResult HitResult))
  (bind _returnvalue (Class|CombatBPI|CanReceiveDamage(Message) _hitactor))
  (if _returnvalue
    (Game|Damage|ApplyPointDamage _hitactor (CallFunction|GetDamage) (Transformation|GetActorForwardVector (Components|GetOwner)) HitResult (Game|GetInstigatorController) self)))

(event EventBeginPlay
  (|CallParentFunction) ; This node is disabled and will not be called.\nDrag off pins to build functionality.
)

(event Collision|EventActorBeginOverlap
  (params (OtherActor :type Actor%20Object%20Reference))
  (|CallParentFunction OtherActor) ; This node is disabled and will not be called.\nDrag off pins to build functionality.
)

(event EventTick
  (params (DeltaSeconds :type Float%20%28single-precision%29))
  (|CallParentFunction DeltaSeconds) ; This node is disabled and will not be called.\nDrag off pins to build functionality.
)

(fn ConstructionScript
  (|CallParentFunction))