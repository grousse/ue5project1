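; Base weapon actor for the combat system, handling equipping, hit damage and per-action montage lookup.
; On equip it attaches to the hand or stowed socket by combat state, registers as main weapon with the owner's combat component and passes its combat type to the AnimInstance.
; Its collision component traces the item mesh, ignoring the owner, and applies point damage to actors that accept it.
; It can also switch the mesh to physics simulation.
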(event OnHit(BP_CollisionComponent)
  (params (HitResult :type Hit%20Result%20Structure))
  (bind _hitactor (Collision|BreakHitResult HitResult))
  ;[1 1 1] OnHit
  (bind _returnvalue (Class|CombatBPI|CanReceiveDamage(Message) _hitactor))
  (if _returnvalue
    (Game|Damage|ApplyPointDamage _hitactor (Variables|Default|GetDamage) (Transformation|GetActorForwardVector (Components|GetOwner)) HitResult (Game|GetInstigatorController) self)))

(event Custom|SimulateWeaponPhysics
  (bind _returnvalue (CallFunction|GetItemMesh))
  ;[1 1 1] SimulateWeaponPhysics
  (Collision|SetCollisionProfileName _returnvalue "PhysicsActor" true :!class /Script/Engine.PrimitiveComponent)
  (Physics|SetSimulatePhysics _returnvalue true))

(event EventBeginPlay
  (|CallParentFunction) ; This node is disabled and will not be called.\nDrag off pins to build functionality.
)

(event Collision|EventActorBeginOverlap
  (params (OtherActor :type Actor%20Object%20Reference))
  (|CallParentFunction OtherActor) ; This node is disabled and will not be called.\nDrag off pins to build functionality.
)

(event EventTick
  (params (DeltaSeconds :type Float%20%28single-precision%29))
  (|CallParentFunction DeltaSeconds) ; This node is disabled and will not be called.\nDrag off pins to build functionality.
)

(fn ConstructionScript
  (|CallParentFunction))

(fn GetSocketName
  (return (Variables|Initialization|GetHandSocketName)))

(fn OnEquiped
  (Variables|Default|SetCombatComponent (Actor|GetComponentbyClass (Components|GetOwner) "/Game/CombatSystem/Blueprints/Components/BP_CombatComponent.BP_CombatComponent_C"))
  (CallFunction|AttachActor (select (Default|IsCombatEnabled? (Variables|Default|GetCombatComponent)) (Variables|Initialization|GetHandSocketName) (Variables|Default|GetAttach%20Socket%20Name)))
  (Default|SetMainWeapon (Variables|Default|GetCombatComponent) self)
  (Class|AnimInstanceBPI|UpdateCombatType(Message) (Components|SkeletalMesh|GetAnimInstance (Variables|/Script/Engine.Character|GetMesh (.AsCharacter (Utilities|Casting|CastToCharacter (Components|GetOwner))))) (Variables|Initialization|GetCombatType))
  (Default|SetCollisionMesh (Variables|Default|GetBP_CollisionComponent) (CallFunction|GetItemMesh))
  (Default|AddActortoIgnore (Variables|Default|GetBP_CollisionComponent) (Components|GetOwner)))

(fn GetActionMontages
  (params (Character%20Action :type E_CharacterAction%20Enum :default "NewEnumerator0"))
  (return (Utilities|Select :Index Character%20Action :NewEnumerator0 0 :NewEnumerator8 0 :NewEnumerator1 (Variables|Montages|GetLigth%20Attack%20Montages) :NewEnumerator2 (Variables|Montages|GetHeavy%20Attack%20Montages) :NewEnumerator9 (Variables|Montages|GetSprint%20Attack%20Montages) :NewEnumerator3 (Variables|Montages|GetCharged%20Attack%20Montages) :NewEnumerator4 (Variables|Montages|GetFalling%20%20Attack%20Montages) :NewEnumerator5 (Variables|Montages|GetDodgeMontages) :NewEnumerator6 (Utilities|Array|MakeArray (Variables|Montages|GetEnterCombat)) :NewEnumerator7 (Utilities|Array|MakeArray (Variables|Montages|GetExitCombat)))))