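; Base Blueprint for dual-wielded weapons, extending a parent weapon with an off-hand mesh and extra collision components for that weapon and the owner's right foot.
; On equip, it binds those components to the off-hand and character meshes, ignores the owner and snaps the off-hand mesh to a socket.
; Toggling combat moves that mesh between hand and attach sockets.
; Collision activation and deactivation route by part to main-weapon, off-hand or foot components.
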(event EventBeginPlay
  (|CallParentFunction) ; This node is disabled and will not be called.\nDrag off pins to build functionality.
)

(event Collision|EventActorBeginOverlap
  (params (OtherActor :type Actor%20Object%20Reference))
  (|CallParentFunction OtherActor) ; This node is disabled and will not be called.\nDrag off pins to build functionality.
)

(event EventTick
  (params (DeltaSeconds :type Float%20%28single-precision%29))
  (|CallParentFunction DeltaSeconds) ; This node is disabled and will not be called.\nDrag off pins to build functionality.
)

(event EventToggleCombat
  (params (bEnableCombat? :type Boolean))
  (|CallParentFunction bEnableCombat?)
  (CallFunction|AttachOff-HandWeapon (select bEnableCombat? (Variables|Initialization|GetSecondWeaponHandSocket) (Variables|Initialization|GetSecondWeaponAttachSocket))))

(fn ConstructionScript
  (|CallParentFunction))

(fn ActivateCollision
  (params (CollisionPart :type E_CollisionPart%20Enum :default "NewEnumerator0"))
  (switch Utilities|FlowControl|Switch|SwitchonE_CollisionPart CollisionPart
    (:NewEnumerator0
      (Default|ActivateCollision (Variables|Default|GetMainWeaponCollisionComponent)))
    (:NewEnumerator1
      (Default|ActivateCollision (Variables|Default|GetOff-HandWeaponCollisionComponent)))
    (:NewEnumerator2
      (Default|ActivateCollision (Variables|Default|GetRightFoot)))))

(fn DeactivateCollision
  (params (Collision%20Part :type E_CollisionPart%20Enum :default "NewEnumerator0"))
  (switch Utilities|FlowControl|Switch|SwitchonE_CollisionPart Collision%20Part
    (:NewEnumerator0
      (Default|DeactivateCollision (Variables|Default|GetMainWeaponCollisionComponent) "NewEnumerator0"))
    (:NewEnumerator1
      (Default|DeactivateCollision (Variables|Default|GetOff-HandWeaponCollisionComponent) "NewEnumerator1"))
    (:NewEnumerator2
      (Default|DeactivateCollision (Variables|Default|GetRightFoot) "NewEnumerator2"))))

(fn OnEquiped
  (|CallParentFunction)
  (Default|SetCollisionMesh (Variables|Default|GetOff-HandWeaponCollisionComponent) (Variables|Default|GetOffHandWeaponMesh))
  (Default|SetCollisionMesh (Variables|Default|GetRightFoot) (Variables|/Script/Engine.Character|GetMesh (.AsCharacter (Utilities|Casting|CastToCharacter (Components|GetOwner)))))
  (CallFunction|AttachOff-HandWeapon (select (Default|IsCombatEnabled? (Variables|Default|GetCombatComponent)) (Variables|Initialization|GetSecondWeaponHandSocket) (Variables|Initialization|GetSecondWeaponAttachSocket)))
  (Default|AddActortoIgnore (Variables|Default|GetOff-HandWeaponCollisionComponent) (Components|GetOwner))
  (Default|AddActortoIgnore (Variables|Default|GetRightFoot) (Components|GetOwner)))

(fn AttachOff-HandWeapon
  (params (Socket :type Name))
  (Transformation|AttachComponentToComponent (Variables|Default|GetOffHandWeaponMesh) (Variables|/Script/Engine.Character|GetMesh (.AsCharacter (Utilities|Casting|CastToCharacter (Components|GetOwner)))) Socket "SnapToTarget" "SnapToTarget" "SnapToTarget" true))