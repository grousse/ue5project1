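; Stats component in the combat system that stores and changes its owner's stat values.
; BaseStats defines a base and max value per stat, and InitializeStats copies the base values into the CurrentStats map.
; ModifyCurrentStatValue adds a delta clamped between zero and the max, while SetCurrentStatValue writes without clamping.
; It has no active events, so initialization relies on an external call.
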(event EventBeginPlay)

(event EventTick
  (params (DeltaSeconds :type Float%20%28single-precision%29)))

(fn GetCurrentStatValue
  (params (Stat :type E_Stats%20Enum :default "NewEnumerator3"))
  (return (.Value (Utilities|Map|Find (Variables|BaseStats|GetCurrentStats) Stat))))

(fn SetCurrentStatValue
  (params (Stat :type E_Stats%20Enum :default "NewEnumerator3") (Value :type Float%20%28double-precision%29))
  (Utilities|Map|Add (Variables|BaseStats|GetCurrentStats) Stat Value))

(fn InitializeStats
  (bind _keys (Utilities|Map|Keys (Variables|BaseStats|GetBaseStats)))
  (for _array_element _keys
    (CallFunction|SetCurrentStatValue _array_element (.basevalue (.Value (Utilities|Map|Find (Variables|BaseStats|GetBaseStats) _array_element))))))

(fn ModifyCurrentStatValue
  (params (Stat :type E_Stats%20Enum :default "NewEnumerator3") (Value :type Float%20%28double-precision%29))
  (if (!= Value 0.0)
    (bind _output_get (LocalVariables|SetL_Value (Math|Float|Clamp(Float) (+ (CallFunction|GetCurrentStatValue Stat) Value) 0.0 (BaseStats|GetMaxStatValue Stat))))
    (CallFunction|SetCurrentStatValue Stat _output_get)))

(fn GetBaseStatValue
  (params (Stat :type E_Stats%20Enum :default "NewEnumerator3"))
  (return (.basevalue (.Value (Utilities|Map|Find (Variables|BaseStats|GetBaseStats) Stat)))))

(fn GetMaxStatValue
  (params (Stat :type E_Stats%20Enum :default "NewEnumerator3"))
  (return (.maxvalue (.Value (Utilities|Map|Find (Variables|BaseStats|GetBaseStats) Stat)))))