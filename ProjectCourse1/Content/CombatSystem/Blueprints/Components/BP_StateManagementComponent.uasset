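; State management component for the combat system that tracks its owner's current state and current character action as two separate values.
; Each setter ignores unchanged values, otherwise firing an end dispatcher for the old value, storing the new one, then firing a begin dispatcher.
; Getters and "equal to any" checks expose both values, and a reset function returns only the state to a default enum entry.
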(event EventBeginPlay)

(event EventTick
  (params (DeltaSeconds :type Float%20%28single-precision%29)))

(fn GetCurrentState
  (return (Variables|Default|GetCurrentState)))

(fn SetState
  (params (New%20State :type E_CharacterState%20Enum :default "NewEnumerator0"))
  (if (Utilities|Enum|NotEqual(Enum) New%20State (Variables|Default|GetCurrentState))
    (Default|CallOnStateEnd (Variables|Default|GetCurrentState))
    (bind _output_get (Variables|Default|SetCurrentState New%20State))
    (Default|CallOnStateBegin _output_get)))

(fn ResetSate
  (CallFunction|SetState "NewEnumerator0"))

(fn IsCurrentStateEqualtoAny
  (params (StatesToCheck :type Array%20of%20E_CharacterState%20Enums :default "NewEnumerator0"))
  (return (Utilities|Array|ContainsItem StatesToCheck (Variables|Default|GetCurrentState))))

(fn GetCurrentAction
  (return (Variables|Default|GetCurrentCharacerAction)))

(fn SetCurrentAction
  (params (New%20Action :type E_CharacterAction%20Enum :default "NewEnumerator0"))
  (if (Utilities|Enum|NotEqual(Enum) New%20Action (Variables|Default|GetCurrentCharacerAction))
    (Default|CallOnCharacterActionEnd (Variables|Default|GetCurrentCharacerAction))
    (bind _output_get (Variables|Default|SetCurrentCharacerAction New%20Action))
    (Default|CallOnCharacterActionBegin _output_get)))

(fn IsCurrentActionEqualtoAny
  (params (ActionsToCheck :type Array%20of%20E_CharacterAction%20Enums :default "NewEnumerator0"))
  (return (Utilities|Array|ContainsItem ActionsToCheck (Variables|Default|GetCurrentCharacerAction))))