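; BP_CollisionComponent is a combat component that detects hits by tracing between two sockets on an assigned collision mesh.
; While collision is enabled, it runs a multi-sphere object trace every Tick, skipping ignored actors.
; An already-hit list, cleared on each enable, lets OnHit fire only once per actor per window.
; Setters and getters expose the mesh, hit state and ignore list.
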(event Custom|EnableCollision
  ;[1 1 1] Enable Collision
  (CallFunction|ClearHitActors)
  (Variables|Default|SetbIsCollisionEnabled? true))

(event Custom|DisableCollision
  ;[1 1 1] Disable collision
  (Variables|Default|SetbIsCollisionEnabled? false))

(event Custom|CollisionTrace
  (bind _collisionmeshcomponent (Variables|Default|GetCollisionMeshComponent))
  ;[1 1 1] Collision Trace
  (bind _outhits (Collision|MultiSphereTraceForObjects (Transformation|GetSocketLocation _collisionmeshcomponent (Variables|Initialization|GetStartSocketName)) (Transformation|GetSocketLocation _collisionmeshcomponent (Variables|Initialization|GetEndSocketName)) (Variables|Initialization|GetTrace%20Radius) (Variables|Initialization|GetCollisionObjectTypes) false (Variables|Default|GetActors%20to%20Ignore) (Variables|Initialization|GetDraw%20Debug%20Type)))
  (for _array_element _outhits
    (bind _output_get (Variables|Default|SetLastHit _array_element))
    (if (not (Utilities|Array|ContainsItem (Variables|Default|GetAlreadyHitActors) (.HitActor (Collision|BreakHitResult _output_get))))
      (bind _output_get_2 (Variables|Default|SetHit%20Actor (.HitActor (Collision|BreakHitResult _output_get))))
      (Utilities|Array|Add (Variables|Default|GetAlreadyHitActors) _output_get_2)
      (Default|CallOnHit (Variables|Default|GetLastHit)))))

(event Custom|ClearHitActors
  ;[1 1 1] Clear hit actors
  (Utilities|Array|Clear (Variables|Default|GetAlreadyHitActors)))

(event Custom|SetCollisionMesh
  (params (CollisionMeshComponent :type Primitive%20Component%20Object%20Reference))
  ;[1 1 1] Set collision mesh component
  (Variables|Default|SetCollisionMeshComponent CollisionMeshComponent))

(event EventBeginPlay)

(event EventTick
  (params (DeltaSeconds :type Float%20%28single-precision%29))
  ;[1 1 1] Collision Trace
  (if (Variables|Default|GetbIsCollisionEnabled?)
    (CallFunction|CollisionTrace)))

(fn GetAlreadyHitActors
  (return (Variables|Default|GetAlreadyHitActors)))

(fn IsCollisionEnabled?
  (return (Variables|Default|GetbIsCollisionEnabled?)))

(fn GetLastHit
  (return (Variables|Default|GetLastHit)))

(fn GetCollisionMeshComponent
  (return (Variables|Default|GetCollisionMeshComponent)))

(fn AddActortoIgnore
  (params (Ignore%20Actor :type Actor%20Object%20Reference%20%28by%20ref%29))
  (Utilities|Array|AddUnique (Variables|Default|GetActors%20to%20Ignore) Ignore%20Actor))

(fn RemoveActortoIgnore
  (params (Actor%20to%20remove :type Actor%20Object%20Reference%20%28by%20ref%29))
  (Utilities|Array|RemoveItem (Variables|Default|GetActors%20to%20Ignore) Actor%20to%20remove))

(fn GetActorstoIgnore
  (return (Variables|Default|GetActors%20to%20Ignore)))