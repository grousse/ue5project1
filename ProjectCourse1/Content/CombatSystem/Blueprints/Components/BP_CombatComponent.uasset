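; BP_CombatComponent is an actor component that holds a character's combat state: main weapon, combat-enabled flag and attack tracking.
; Setting a new main weapon calls OnUnequiped on the current one and destroys it before storing the replacement.
; Toggling combat stores the flag and forwards it to the owning Character's anim instance through an UpdateCombatEnabledMessage call.
; Resetting an attack zeroes the attack count and clears the saved-attack flag.
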(event EventBeginPlay)

(event EventTick
  (params (DeltaSeconds :type Float%20%28single-precision%29)))

(fn SetMainWeapon
  (params (New%20Weapon :type BP%20Base%20Weapon%20Object%20Reference))
  (Utilities|FlowControl|Sequence
    (:then_0
      (Utilities|IsValid (Variables|Default|GetMainWeapon)
        (:Is%20Valid
          (Default|OnUnequiped (Variables|Default|GetMainWeapon))
          (Actor|DestroyActor (Variables|Default|GetMainWeapon)))))
    (:then_1
      (Variables|Default|SetMainWeapon New%20Weapon))))

(fn GetMainWeapon
  (return (Variables|Default|GetMainWeapon)))

(fn SetCombatEnabled
  (params (bCombatEnabled? :type Boolean))
  (bind _output_get (Variables|Default|SetbCombatEnabled? bCombatEnabled?))
  (Class|AnimInstanceBPI|UpdateCombatEnabled(Message) (Components|SkeletalMesh|GetAnimInstance (Variables|/Script/Engine.Character|GetMesh (.AsCharacter (Utilities|Casting|CastToCharacter (Components|GetOwner))))) _output_get))

(fn IsCombatEnabled?
  (return (Variables|Default|GetbCombatEnabled?)))

(fn ResetAttack
  (Variables|Default|SetAttackCount 0)
  (Variables|Default|SetbIsAttackSaved? false))