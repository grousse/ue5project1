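; Test dummy character for the combat system that takes point damage and shows hit feedback.
; On BeginPlay it initializes its stats component, then spawns and equips each starting equipment class.
; Point damage goes to the stats component and triggers an impact sound and explosion particle at the hit location.
; When a hit reaction is allowed, it plays a front-react montage and changes state through the state management component.
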(event EventBeginPlay
  (bind _self self)
  (Default|InitializeStats (Variables|Default|GetStatsComponent))
  (for _array_element (Variables|Default|GetStartingEquipment)
    (bind _returnvalue (Game|SpawnActorfromClass _array_element (Transformation|GetActorTransform) "Undefined" _self _self))
    (Default|OnEquiped _returnvalue)))

(event Collision|EventActorBeginOverlap
  (params (OtherActor :type Actor%20Object%20Reference)))

(event EventTick
  (params (DeltaSeconds :type Float%20%28single-precision%29)))

(event Game|Damage|EventPointDamage
  (params (Damage :type Float%20%28single-precision%29) (DamageType :type Damage%20Type%20Object%20Reference) (HitLocation :type Vector :default "0, 0, 0") (HitNormal :type Vector :default "0, 0, 0") (HitComponent :type Primitive%20Component%20Object%20Reference) (BoneName :type Name :default "None") (ShotFromDirection :type Vector :default "0, 0, 0") (InstigatedBy :type Controller%20Object%20Reference) (DamageCauser :type Actor%20Object%20Reference) (HitInfo :type Hit%20Result%20Structure%20%28by%20ref%29))
  ;[1 1 1] PointDamage
  (Default|TakeDamage (Variables|Default|GetStatsComponent) Damage)
  (Audio|PlaySoundatLocation "/Game/CombatSystem/CourseFiles/Meshes/SoundFX/Gruntling/A_Guardian_Impact_Cue.A_Guardian_Impact_Cue" HitLocation "0, 0, 0" 1.0 1.0 0.0 0 0 0 0)
  (Effects|SpawnEmitteratLocation "/Game/StarterContent/Particles/P_Explosion.P_Explosion" HitLocation)
  (if (CallFunction|CanReceiveHitReaction)
    (Animation|PlayAnimMontage "/Game/Characters/Mannequin_UE4/UE4_MannyAnims/Standing_React_Large_Front_Montage.Standing_React_Large_Front_Montage" 1.0 "None")
    (Default|SetState (Variables|Default|GetStateManagementComponent) "NewEnumerator5")))

(fn ConstructionScript
  (|CallParentFunction))